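; BP_BaseFloor is a floor actor that holds a logic number and displays it on a text render component.
; The construction script creates a dynamic instance of the cube material, stores it and sets its Color parameter to green.
; The number is written to the text at construction and BeginPlay, and SetLogicNum updates both the stored value and the label.
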(event `self.ReceiveBeginPlay`
  (`TextRenderComponent.K2_SetText` (`self.TextRender`) (`KismetTextLibrary.Conv_IntToText` (`self.LogicNum`))))

(fn `SetLogicNum`
  (params (Num :type Integer))
  (set `self.LogicNum` Num)
  (`TextRenderComponent.K2_SetText` (`self.TextRender`) (`KismetTextLibrary.Conv_IntToText` (`self.LogicNum`))))

(fn `UserConstructionScript`
  (bind _returnvalue (`KismetMaterialLibrary.CreateDynamicMaterialInstance` "/Game/Geometry/Meshes/CubeMaterial.CubeMaterial"))
  (bind _output_get (set `self.Mat` _returnvalue))
  (`MaterialInstanceDynamic.SetVectorParameterValue` _output_get "Color" (struct :`R` 0.318574 :`G` 1.0 :`A` 1.0))
  (`TextRenderComponent.K2_SetText` (`self.TextRender`) (`KismetTextLibrary.Conv_IntToText` (`self.LogicNum`))))